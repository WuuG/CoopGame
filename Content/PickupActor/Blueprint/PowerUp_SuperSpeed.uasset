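; Super-speed power-up pickup that temporarily boosts the walk speed of the first player's pawn.
; On activation it doubles the CharacterMovementComponent's MaxWalkSpeed, then calls the parent handler.
; On expiry it halves the current speed to undo the boost, destroys itself and calls the parent handler; timing is not handled in this Blueprint.
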(event EventOnActivated
  (bind _returnvalue (Game|Player|GetPlayerPawn 0))
  (bind _returnvalue_2 (Actor|GetComponentbyClass _returnvalue "/Script/Engine.CharacterMovementComponent"))
  (Variables|/Script/Engine.CharacterMovementComponent|SetMaxWalkSpeed _returnvalue_2 (* (Variables|/Script/Engine.CharacterMovementComponent|GetMaxWalkSpeed _returnvalue_2) 2.0))
  (|CallParentFunction))

(event EventOnExpired
  (bind _returnvalue (Game|Player|GetPlayerPawn 0))
  (bind _returnvalue_2 (Actor|GetComponentbyClass _returnvalue "/Script/Engine.CharacterMovementComponent"))
  (Variables|/Script/Engine.CharacterMovementComponent|SetMaxWalkSpeed _returnvalue_2 (/ (Variables|/Script/Engine.CharacterMovementComponent|GetMaxWalkSpeed _returnvalue_2) 2.0))
  (Actor|DestroyActor)
  (|CallParentFunction))

(fn ConstructionScript)
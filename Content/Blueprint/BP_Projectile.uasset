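; BP_Projectile is an explosive projectile that detonates one second after spawning, or earlier when it overlaps a BP_TargetDummy.
; Both triggers call Expolde, which spawns an explosion emitter, applies full radial damage blockable on the Pawn channel and destroys the actor.
; Damage is always credited to player controller 0.
; The COOP.DebugWeapons console variable enables a debug sphere showing the damage radius.
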(event Custom|Expolde
  (bind _returnvalue (Transformation|GetActorLocation))
  (Effects|SpawnEmitteratLocation "/Game/WeaponEffects/Explosion/P_Explosion.P_Explosion" _returnvalue)
  (Game|Damage|ApplyRadialDamage 1e+02 _returnvalue (Variables|Default|GetDamage%20Radius) 0 0 self (Game|GetPlayerController 0) true "ECC_Pawn")
  (Actor|DestroyActor)
  (bind _returnvalue_2 (Development|GetConsoleVariableIntValue "COOP.DebugWeapons"))
  (Math|Integer|CompareInt _returnvalue_2
    (:>
      (Rendering|Debug|DrawDebugSphere (Transformation|GetActorLocation) (Variables|Default|GetDamage%20Radius) 12 "(R=1.000000,G=0.000000,B=0.911144,A=1.000000)" 1.0 2.0))))

(event Collision|EventActorBeginOverlap
  (params (OtherActor :type Actor%20Object%20Reference))
  (Utilities|Casting|CastToBP_TargetDummy OtherActor)
  (CallFunction|Expolde))

(event EventBeginPlay
  (Utilities|FlowControl|Delay 1.0)
  (CallFunction|Expolde))

(fn ConstructionScript)